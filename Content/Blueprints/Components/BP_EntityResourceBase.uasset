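; Base component for an entity resource, tracking a current value against a maximum and starting full on BeginPlay.
; IncreaseValue adds up to the maximum, or fills it outright when IsClamped is set, while DecreaseValue rejects amounts exceeding the current value.
; Changes fire event dispatchers: OnValueIncreased also covers non-zero decreases, and OnZeroValue signals depletion.
; Tick prints current and maximum values on screen for debugging.
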(event EventBeginPlay
  (CallFunction|ConfigureValue))

(event EventTick
  (params (DeltaSeconds :type Float%20%28single-precision%29))
  (CallFunction|Debug))

(fn IncreaseValue
  (params (IsClamped :type Boolean) (Amount :type Float%20%28single-precision%29))
  (if (< (Variables|Default|GetCurrentValue) (Variables|Default|GetMaxValue))
    (if (> Amount 0.0)
      (if (not IsClamped)
        (bind _output_get (Variables|Default|SetCurrentValue (Math|Float|Min(Float) (+ (Variables|Default|GetCurrentValue) Amount) (Variables|Default|GetMaxValue))))
        (Default|CallOnValueIncreased _output_get)
        (return true)
        (else
          (bind _output_get_2 (Variables|Default|SetCurrentValue (Variables|Default|GetMaxValue)))
          (Default|CallOnValueIncreased _output_get_2)
          (return false)))
      (else
        (return false)))
    (else
      (return false))))

(fn DecreaseValue
  (params (Amount :type Float%20%28single-precision%29))
  (if (and (> Amount 0.0) (>= (Variables|Default|GetCurrentValue) Amount))
    (bind _output_get (Variables|Default|SetCurrentValue (Math|Float|Max(Float) (- (Variables|Default|GetCurrentValue) Amount) 0.0)))
    (if (> _output_get 0.0)
      (Default|CallOnValueIncreased (Variables|Default|GetCurrentValue))
      (return true)
      (else
        (Default|CallOnZeroValue)
        (return true)))
    (else
      (return false))))

(fn ConfigureValue
  (bind _output_get (Variables|Default|SetCurrentValue (Variables|Default|GetMaxValue)))
  (Default|CallOnValueIncreased _output_get))

(fn Debug
  (Development|PrintString (Utilities|String|Append (Utilities|String|ToString(Float) (Variables|Default|GetCurrentValue)) " || " (Utilities|String|ToString(Float) (Variables|Default|GetMaxValue))) true true "(R=0.916354,G=0.000000,B=1.000000,A=1.000000)" 0.0))