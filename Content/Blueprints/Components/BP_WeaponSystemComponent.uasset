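; Weapon inventory component for BP_CharacterBase owners that spawns, equips and switches the character's weapons.
; On BeginPlay it spawns each weapon class hidden on the backpack socket, then equips the current index.
; Equipping moves that weapon to the hand socket, broadcasts the change with its icon, activates it and deactivates the previous one.
; Switching works by index or wrap-around cycling, ammo pickups map to fixed slots, and Tick runs the current weapon's debug.
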(event EventBeginPlay
  (CallFunction|SpawnWeapon)
  (CallFunction|EquipWeapon))

(event EventTick
  (params (DeltaSeconds :type Float%20%28single-precision%29))
  (Default|Debug (Variables|Default|GetCurrentWeapon) DeltaSeconds))

(fn SwitchWeapon
  (params (WeaponIndex :type Integer))
  (if (!= WeaponIndex (Variables|Default|GetCurrentWeaponIndex))
    (Variables|Default|SetCurrentWeaponIndex WeaponIndex)
    (CallFunction|EquipWeapon (Variables|Default|GetCurrentWeapon))
    (else
      (Development|PrintString "Hello"))))

(fn EquipWeapon
  (params (L_CurrentWeapon :type BP%20Weapon%20Base%20Object%20Reference))
  (bind _weaponactors (Variables|Default|GetWeaponActors))
  (bind _currentweaponindex (Variables|Default|GetCurrentWeaponIndex))
  (bind _output (Utilities|Array|Get(acopy) _weaponactors _currentweaponindex))
  (if (> (Utilities|Array|Length (Variables|Default|GetWeaponActors)) 0)
    (Utilities|IsValid _output
      (:Is%20Valid
        (bind _output_get (Variables|Default|SetCurrentWeapon _output))
        (Default|CallOnWeaponChange _output_get (Utilities|Struct|BreakSTRUCT_WeaponStats (Variables|/Game/Weapons/BP_WeaponBase.BP_WeaponBase_C|GetWeaponStats (Variables|Default|GetCurrentWeapon))))
        (CallFunction|AttachWeapon (Variables|Default|GetCurrentWeapon) (Variables|Socket|GetHandPointSocket))
        (bind _currentweapon (Variables|Default|GetCurrentWeapon)
          (:then
            (Default|ActivateWeapon _currentweapon)
            (bind _l_currentweapon (LocalVariables|GetL_CurrentWeapon)
              (:then
                (Default|DeactivateWeapon _l_currentweapon))
              (:else)))
          (:else))))))

(fn SpawnWeapon
  (|SetOwnerMesh)
  (for _array_element (Variables|Default|GetWeaponClass)
    (bind _returnvalue (Game|SpawnActorfromClass _array_element (Transformation|GetWorldTransform (Variables|Default|GetOwnerMesh)) "AdjustIfPossibleButAlwaysSpawn" (Components|GetOwner) 0))
    (Utilities|IsValid _returnvalue
      (:Is%20Valid
        (bind _output_get (LocalVariables|SetL_SpawnedWeapon _returnvalue))
        (Utilities|Array|Add (Variables|Default|GetWeaponActors) _output_get)
        (CallFunction|AttachWeapon (LocalVariables|GetL_SpawnedWeapon) (Variables|Socket|GetBackPackSocket))
        (bind _l_spawnedweapon (LocalVariables|GetL_SpawnedWeapon)
          (:then
            (Rendering|SetVisibility (Variables|/Game/Weapons/BP_WeaponBase.BP_WeaponBase_C|GetSkeletalMesh _l_spawnedweapon) false false))
          (:else)))))
  (return))

(fn AttachWeapon
  (params (Weapon :type Actor%20Object%20Reference) (SocketName :type Name))
  (Transformation|AttachComponentToComponent Weapon (Variables|Default|GetOwnerMesh) SocketName "SnapToTarget" "KeepWorld" "SnapToTarget" true))

(fn SwitchtoNext
  (bind _output_get (LocalVariables|SetL_CurrentIndex (Math|Integer|%(Integer) (+ (Variables|Default|GetCurrentWeaponIndex) 1) (Utilities|Array|Length (Variables|Default|GetWeaponActors)))))
  (Variables|Default|SetCurrentWeaponIndex _output_get)
  (CallFunction|EquipWeapon (Variables|Default|GetCurrentWeapon))
  (return))

(fn StartAmmoIncrease
  (params (AmmoType :type ENUM_AmmoType%20Enum :default "NewEnumerator0") (AmmoValue :type Integer))
  (bind _success (Default|IncreaseAmmo (Utilities|Select :Index AmmoType :NewEnumerator0 (Utilities|Array|Get(acopy) (Variables|Default|GetWeaponActors)) :NewEnumerator1 (Utilities|Array|Get(acopy) (Variables|Default|GetWeaponActors) 1)) AmmoValue))
  (return _success))

(fn GetCurrentWeapon
  (bind _currentweapon (Variables|Default|GetCurrentWeapon)
    (:then
      (return _currentweapon))
    (:else)))