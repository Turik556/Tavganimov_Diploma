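; BP_DamageTrigger is a trigger object that damages the actor overlapping it.
; Overlap events forward to the parent class, and its OverlappEffect override runs the parent effect, then applies Damage to a valid OverlappedActor using the BP_DamageObject damage type.
; The override returns whether that actor was valid, and Interact always returns false.
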(event EventBeginPlay
  (|CallParentFunction) ; This node is disabled and will not be called.\nDrag off pins to build functionality.
)

(event Collision|EventActorBeginOverlap
  (params (OtherActor :type Actor%20Object%20Reference))
  (|CallParentFunction OtherActor))

(event EventTick
  (params (DeltaSeconds :type Float%20%28single-precision%29))
  (|CallParentFunction DeltaSeconds) ; This node is disabled and will not be called.\nDrag off pins to build functionality.
)

(fn ConstructionScript
  (|CallParentFunction))

(fn OverlappEffect
  (|CallParentFunction)
  (bind _overlappedactor (Variables|Default|GetOverlappedActor)
    (:then
      (Game|Damage|ApplyDamage _overlappedactor (Variables|Default|GetDamage) 0 self "/Game/Blueprints/Objects/BP_DamageObject.BP_DamageObject_C")
      (return true))
    (:else
      (return false))))

(fn Interact
  (params (Actor :type Actor%20Object%20Reference))
  (return false))