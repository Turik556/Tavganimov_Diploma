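; Base door Blueprint that swings open and shut by rotating DoorRotator's yaw.
; OpenDoor and CloseDoor play one timeline forward or in reverse, scaled by OpenDoorAngle and blocked while in progress; finishing toggles IsDoorOpen.
; The collision box records the overlapping actor but triggers no movement, and a dot-product check for swing direction is left unconnected.
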(event OnComponentBeginOverlap(CollissionBox)
  (params (OverlappedComponent :type Primitive%20Component%20Object%20Reference) (OtherActor :type Actor%20Object%20Reference) (OtherComp :type Primitive%20Component%20Object%20Reference) (OtherBodyIndex :type Integer) (bFromSweep :type Boolean) (SweepResult :type Hit%20Result%20Structure%20%28by%20ref%29))
  (Utilities|IsValid OtherActor
    (:Is%20Valid
      (Variables|Default|SetOverlappedActor OtherActor))))

(event OnComponentEndOverlap(CollissionBox)
  (params (OverlappedComponent :type Primitive%20Component%20Object%20Reference) (OtherActor :type Actor%20Object%20Reference) (OtherComp :type Primitive%20Component%20Object%20Reference) (OtherBodyIndex :type Integer)))

(event Custom|OpenDoor
  (if (not (Variables|Default|GetIsInProgress))
    (bind _doortimer (Timeline|Timeline_0 PlayFromStart)
      (:Update
        (Variables|Default|SetIsInProgress true)
        (Transformation|SetRelativeRotation (Variables|Default|GetDoorRotator) (Math|Rotator|MakeRotator 0.0 0.0 (* _doortimer (Variables|Default|GetOpenDoorAngle))) false false))
      (:Finished
        (Variables|Default|SetIsInProgress false)
        (if (not (Variables|Default|GetIs%20DoorOpen))
          (Variables|Default|SetIs%20DoorOpen true)
          (else
            (Variables|Default|SetIs%20DoorOpen false)))))))

(event Custom|CloseDoor
  (if (not (Variables|Default|GetIsInProgress))
    (bind _doortimer (Timeline|Timeline_0 ReverseFromEnd)
      (:Update
        (Variables|Default|SetIsInProgress true)
        (Transformation|SetRelativeRotation (Variables|Default|GetDoorRotator) (Math|Rotator|MakeRotator 0.0 0.0 (* _doortimer (Variables|Default|GetOpenDoorAngle))) false false))
      (:Finished
        (Variables|Default|SetIsInProgress false)
        (if (not (Variables|Default|GetIs%20DoorOpen))
          (Variables|Default|SetIs%20DoorOpen true)
          (else
            (Variables|Default|SetIs%20DoorOpen false)))))))

(event EventBeginPlay)

(event Collision|EventActorBeginOverlap
  (params (OtherActor :type Actor%20Object%20Reference)))

(event EventTick
  (params (DeltaSeconds :type Float%20%28single-precision%29)))

(fn ConstructionScript)