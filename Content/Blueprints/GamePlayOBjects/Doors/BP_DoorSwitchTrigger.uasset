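; Door switch trigger that toggles a set of target doors when an actor begins overlapping it.
; After running the parent overlap logic, it calls InteractWithDoor, which loops over the valid TargetDoors and opens or closes each based on its own IsDoorOpen state.
; The overlapping actor is not filtered here, and there is no end-overlap handling, so each new overlap flips the doors again.
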(event EventBeginPlay
  (|CallParentFunction) ; This node is disabled and will not be called.\nDrag off pins to build functionality.
)

(event Collision|EventActorBeginOverlap
  (params (OtherActor :type Actor%20Object%20Reference))
  (|CallParentFunction OtherActor)
  (CallFunction|InteractwithDoor))

(event EventTick
  (params (DeltaSeconds :type Float%20%28single-precision%29))
  (|CallParentFunction DeltaSeconds) ; This node is disabled and will not be called.\nDrag off pins to build functionality.
)

(fn ConstructionScript
  (|CallParentFunction))

(fn InteractwithDoor
  (for _array_element (Variables|Default|GetTargetDoors)
    (Utilities|IsValid _array_element
      (:Is%20Valid
        (bind _output_get (LocalVariables|SetL_TargetDoor _array_element))
        (if (Variables|/Game/Blueprints/GamePlayOBjects/Doors/BP_DoorBase.BP_DoorBase_C|GetIs%20DoorOpen _output_get)
          (Default|CloseDoor (LocalVariables|GetL_TargetDoor))
          (else
            (Default|OpenDoor (LocalVariables|GetL_TargetDoor))))))))