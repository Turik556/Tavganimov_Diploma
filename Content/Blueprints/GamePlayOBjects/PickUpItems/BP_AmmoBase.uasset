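; BP_AmmoBase is a base ammo pickup item that adds ammo to the weapon of the actor that picks it up.
; Its PickUpEffect finds the actor's BP_WeaponSystemComponent and calls IncreaseAmmo on the current weapon with AmmoValue.
; It returns that call's result, or false when the actor, component or weapon is invalid.
; The event graph holds only disabled default events, so all logic lives in PickUpEffect.
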(event EventBeginPlay
  (|CallParentFunction) ; This node is disabled and will not be called.\nDrag off pins to build functionality.
)

(event Collision|EventActorBeginOverlap
  (params (OtherActor :type Actor%20Object%20Reference))
  (|CallParentFunction OtherActor) ; This node is disabled and will not be called.\nDrag off pins to build functionality.
)

(event EventTick
  (params (DeltaSeconds :type Float%20%28single-precision%29))
  (|CallParentFunction DeltaSeconds) ; This node is disabled and will not be called.\nDrag off pins to build functionality.
)

(fn ConstructionScript
  (|CallParentFunction))

(fn PickUpEffect
  (params (Actor :type Actor%20Object%20Reference))
  (bind _returnvalue (Actor|GetComponentbyClass Actor "/Game/Blueprints/Components/BP_WeaponSystemComponent.BP_WeaponSystemComponent_C"))
  (bind _currentweapon (Variables|/Game/Blueprints/Components/BP_WeaponSystemComponent.BP_WeaponSystemComponent_C|GetCurrentWeapon _returnvalue))
  (Utilities|IsValid Actor
    (:Is%20Valid
      (Utilities|IsValid _returnvalue
        (:Is%20Valid
          (Utilities|IsValid _currentweapon
            (:Is%20Valid
              (bind _success (Default|IncreaseAmmo _currentweapon (Variables|Default|GetAmmoValue)))
              (return _success))
            (:Is%20Not%20Valid
              _)))
        (:Is%20Not%20Valid
          _)))
    (:Is%20Not%20Valid
      _))
  (return false))