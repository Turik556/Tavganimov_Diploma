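; BP_KeyBase is a base pickup item for keys that grants a key to the actor that picks it up.
; Its PickUpEffect override calls the parent, then looks for a BP_KeyHolder_Component on that actor and adds its KeyType through AddKey.
; It returns the AddKey result, or false when the actor is invalid or has no key holder component.
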(event EventBeginPlay
  (|CallParentFunction) ; This node is disabled and will not be called.\nDrag off pins to build functionality.
)

(event Collision|EventActorBeginOverlap
  (params (OtherActor :type Actor%20Object%20Reference))
  (|CallParentFunction OtherActor) ; This node is disabled and will not be called.\nDrag off pins to build functionality.
)

(event EventTick
  (params (DeltaSeconds :type Float%20%28single-precision%29))
  (|CallParentFunction DeltaSeconds) ; This node is disabled and will not be called.\nDrag off pins to build functionality.
)

(fn ConstructionScript
  (|CallParentFunction))

(fn PickUpEffect
  (params (Actor :type Actor%20Object%20Reference))
  (bind _returnvalue (Actor|GetComponentbyClass Actor "/Game/Characters/PlayerCharacter/Components/BP_KeyHolder_Component.BP_KeyHolder_Component_C"))
  (|CallParentFunction Actor)
  (Utilities|IsValid Actor
    (:Is%20Valid
      (Utilities|IsValid _returnvalue
        (:Is%20Valid
          (bind _success (Default|AddKey _returnvalue (Variables|Default|GetKeyType)))
          (return _success))
        (:Is%20Not%20Valid
          (return false))))
    (:Is%20Not%20Valid
      (return false))))