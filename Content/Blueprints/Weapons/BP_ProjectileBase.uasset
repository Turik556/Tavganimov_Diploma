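; BP_ProjectileBase is a weapon projectile that launches along MovementDirection at the movement component's initial speed on BeginPlay.
; On a sphere hit it prints the other actor's name, applies fixed damage if that actor's class exactly equals BP_CharacterBase, then destroys itself.
; SetTargetLocation traces from the player camera but leaves the result unused, and SpawnDecal only spawns an emitter; neither is called here.
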(event OnComponentHit(Sphere)
  (params (HitComponent :type Primitive%20Component%20Object%20Reference) (OtherActor :type Actor%20Object%20Reference) (OtherComp :type Primitive%20Component%20Object%20Reference) (NormalImpulse :type Vector :default "0, 0, 0") (Hit :type Hit%20Result%20Structure%20%28by%20ref%29))
  (Development|PrintString (Utilities|GetDisplayName OtherActor))
  (if (== (Utilities|GetClass OtherActor) "/Game/Characters/BP_CharacterBase.BP_CharacterBase_C")
    (Game|Damage|ApplyDamage 0 5.0 0 0))
  (Actor|DestroyActor))

(event EventBeginPlay
  (Variables|/Script/Engine.MovementComponent|SetVelocity (Variables|Default|GetProjectileMovement) (* (Variables|Default|GetMovement%20Direction) (Variables|/Script/Engine.ProjectileMovementComponent|GetInitialSpeed (Variables|Default|GetProjectileMovement)))))

(event EventTick
  (params (DeltaSeconds :type Float%20%28single-precision%29)))

(fn ConstructionScript)

(fn SetTargetLocation
  (bind _returnvalue (Game|GetPlayerCharacter 0))
  (Utilities|IsValid _returnvalue
    (:Is%20Valid
      (bind _asbp_player_character (Utilities|Casting|CastToBP_PlayerCharacter _returnvalue))
      (bind _desiredview (Class|CameraComponent|GetCameraView (Variables|/Game/Characters/PlayerCharacter/BP_PlayerCharacter.BP_PlayerCharacter_C|GetCamera _asbp_player_character) 0.0))
      (bind _outhit (Collision|LineTraceByChannel (Utilities|Struct|BreakMinimalViewInfo _desiredview) (+ (Utilities|Struct|BreakMinimalViewInfo _desiredview) (* (Math|Vector|GetForwardVector (Variables|/Game/Characters/PlayerCharacter/BP_PlayerCharacter.BP_PlayerCharacter_C|GetCamera _asbp_player_character)) 5e+03)) "TraceTypeQuery2" false 0 "ForDuration")))))

(fn SpawnDecal
  (params (Hit :type Hit%20Result%20Structure))
  (Effects|SpawnEmitteratLocation 0 "0, 0, 0"))