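; Base weapon actor handling firing, ammunition and reloading, configured through a WeaponStats struct and tracked by a weapon state enum.
; Shooting traces from the owner's camera, then either spawns a projectile aimed from the muzzle at the trace point or applies hitscan damage.
; Automatic weapons set a looping timer from rate of fire.
; Shots drain the magazine and signal when empty, while reloading refills it from reserve ammo.
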(event EventBeginPlay)

(event Collision|EventActorBeginOverlap
  (params (OtherActor :type Actor%20Object%20Reference)))

(event EventTick
  (params (DeltaSeconds :type Float%20%28single-precision%29)))

(fn ConstructionScript)

(fn HasAmmo
  (return (> (.Ammo (Utilities|Struct|BreakSTRUCT_WeaponStats (Variables|Default|GetWeaponStats))) 0)))

(fn ReloadMagazine
  (bind _weaponstats (Variables|Default|GetWeaponStats))
  (bind _weaponstats_2 (Variables|Default|GetWeaponStats))
  (bind _weaponstats_3 (Variables|Default|GetWeaponStats))
  (bind _weaponstats_4 (Variables|Default|GetWeaponStats))
  (bind _maxmagazimeammo (Utilities|Struct|BreakSTRUCT_WeaponStats _weaponstats))
  (bind _ammo (Utilities|Struct|BreakSTRUCT_WeaponStats _weaponstats_4))
  (bind (_ammo_2 _maxmagazimeammo_2) (Utilities|Struct|BreakSTRUCT_WeaponStats _weaponstats_2))
  (bind (_maxmagazimeammo_3 _currentammo) (Utilities|Struct|BreakSTRUCT_WeaponStats _weaponstats_3))
  (if (Ammo|HasAmmo)
    (if (MagazineAmmo|IsEnoughAmmo)
      (Ammo|DecreaseAmmo (- _maxmagazimeammo_3 _currentammo))
      (Utilities|Struct|SetmembersinSTRUCT_WeaponStats _weaponstats_3 _maxmagazimeammo_3)
      (return true)
      (else
        (if (> _ammo_2 _maxmagazimeammo_2)
          (Utilities|Struct|SetmembersinSTRUCT_WeaponStats _weaponstats _maxmagazimeammo)
          (Ammo|DecreaseAmmo _maxmagazimeammo)
          (else
            (Utilities|Struct|SetmembersinSTRUCT_WeaponStats _weaponstats_4 _ammo)
            (Ammo|DecreaseAmmo _ammo)))
        (return true)))
    (else
      (return false))))

(fn IncreaseAmmo
  (params (Value :type Integer))
  (bind _weaponstats (Variables|Default|GetWeaponStats))
  (if (> Value 0)
    (Utilities|Struct|SetmembersinSTRUCT_WeaponStats _weaponstats (+ (.Ammo (Utilities|Struct|BreakSTRUCT_WeaponStats _weaponstats)) Value))
    (return true)
    (else
      (return false))))

(fn DecreaseMagazineAmmo
  (bind _weaponstats (Variables|Default|GetWeaponStats))
  (Utilities|Struct|SetmembersinSTRUCT_WeaponStats _weaponstats (Math|Integer|Max(Integer) (- (.CurrentAmmo (Utilities|Struct|BreakSTRUCT_WeaponStats _weaponstats)) 1)))
  (if (MagazineAmmo|IsEnoughAmmo)
    _
    (else
      (Default|CallOnAmmoRunOut)))
  (return))

(fn IsEnoughAmmo
  (return (> (.CurrentAmmo (Utilities|Struct|BreakSTRUCT_WeaponStats (Variables|Default|GetWeaponStats))) 0)))

(fn DecreaseAmmo
  (params (Value :type Integer))
  (bind _weaponstats (Variables|Default|GetWeaponStats))
  (Utilities|Struct|SetmembersinSTRUCT_WeaponStats _weaponstats (Math|Integer|Max(Integer) (- (.Ammo (Utilities|Struct|BreakSTRUCT_WeaponStats _weaponstats)) Value)))
  (return))

(fn Reload
  (if (Ammo|HasAmmo)
    ;[1 1 1] Placeholder for Reload animation
    (Variables|Default|SetWeaponState "NewEnumerator0")
    (bind _success (MagazineAmmo|ReloadMagazine))
    (Variables|Default|SetCanShoot _success)
    (Default|CallOnAmmoReload)))

(fn StartShooting
  (if (Variables|Default|GetCanShoot)
    (Variables|Default|SetWeaponState "NewEnumerator1")
    (|GetOwnerCamera)
    (Shooting|MakeShot)
    (Utilities|IsAuto
      (:true
        (if (MagazineAmmo|IsEnoughAmmo)
          (bind _timebetweenshots (CallFunction|CalculateTimeBetweenShots))
          (Utilities|Time|SetTimerbyEvent (EventDispatchers|CreateEvent :!event MakeShot) _timebetweenshots true)))
      (:false
        _))
    (return)
    (else
      (return))))

(fn MakeShot
  (if (Utilities|Enum|Equal(Enum) (Variables|Default|GetWeaponState) "NewEnumerator1")
    (bind (_hitactor _movementdirection) (CallFunction|SetTargetLocation))
    (Utilities|SwithShootType
      (:Projectile
        (bind _returnvalue (Game|SpawnActorfromClass (.ProjectileClass (Utilities|Struct|BreakSTRUCT_WeaponStats (Variables|Default|GetWeaponStats))) (Transformation|GetWorldTransform (Variables|Default|GetMuzzleScene)) "Undefined" self (.DamageValue (Utilities|Struct|BreakSTRUCT_WeaponStats (Variables|Default|GetWeaponStats))) _movementdirection self 0))
        (Utilities|IsValid _returnvalue
          (:Is%20Valid
            (LocalVariables|SetL_Projectile _returnvalue)
            (MagazineAmmo|DecreaseMagazineAmmo)
            (return))))
      (:Hitscan
        (Game|Damage|ApplyDamage _hitactor (Math|Conversions|ToFloat(Integer) (.DamageValue (Utilities|Struct|BreakSTRUCT_WeaponStats (Variables|Default|GetWeaponStats)))) 0 self "/Game/Blueprints/Objects/BP_DamageObject.BP_DamageObject_C")
        (MagazineAmmo|DecreaseMagazineAmmo)
        (return)))))

(fn ActivateWeapon
  (Variables|Default|SetWeaponState "NewEnumerator2")
  (Rendering|SetVisibility (Variables|Default|GetSkeletalMesh) true false)
  (EventDispatchers|BindEventtoOnAmmoRunOut (EventDispatchers|CreateEvent :!event NeedReload))
  (Variables|Default|SetCanShoot true))

(fn DeactivateWeapon
  (Variables|Default|SetWeaponState "NewEnumerator4")
  (Rendering|SetVisibility (Variables|Default|GetSkeletalMesh) false false)
  (EventDispatchers|UnbindEventfromOnAmmoRunOut (EventDispatchers|CreateEvent :!event Reload)))

(fn Debug
  (params (Duration :type Float%20%28single-precision%29))
  (bind _weaponstats (Variables|Default|GetWeaponStats))
  (bind (_ammo _maxmagazimeammo _currentammo) (Utilities|Struct|BreakSTRUCT_WeaponStats _weaponstats))
  (Development|PrintString (Utilities|String|Append (Utilities|String|ToString(Integer) _currentammo) " |" (Utilities|String|ToString(Integer) _maxmagazimeammo) " || " (Utilities|String|ToString(Integer) _ammo)) true true "(R=0.000000,G=0.660000,B=1.000000,A=1.000000)" Duration)
  (Development|PrintString (Utilities|String|EnumtoString (Variables|Default|GetWeaponState)) true true "(R=1.000000,G=0.035352,B=0.000000,A=1.000000)" Duration))

(fn NeedReload
  (Variables|Default|SetWeaponState "NewEnumerator5")
  (Variables|Default|SetCanShoot false))

(fn SetTargetLocation
  (bind _desiredview (Class|CameraComponent|GetCameraView (Variables|Default|GetOwnerCameraComponent) 0.0))
  (LocalVariables|SetL_StartPoint (Utilities|Struct|BreakMinimalViewInfo _desiredview))
  (LocalVariables|SetL_EndPoint (+ (LocalVariables|GetL_StartPoint) (* (Math|Vector|GetForwardVector (Variables|Default|GetOwnerCameraComponent)) (LocalVariables|GetTraceLenght))))
  (bind _outhit (Collision|LineTraceByChannel (LocalVariables|GetL_StartPoint) (LocalVariables|GetL_EndPoint) "TraceTypeQuery3" false (Utilities|Array|MakeArray (Components|GetOwner)) "ForDuration"))
  (LocalVariables|SetL_HitActor (.HitActor (Collision|BreakHitResult _outhit)))
  (return (LocalVariables|GetL_HitActor) (Math|Vector|Normalize (- (select (.bBlockingHit (Collision|BreakHitResult _outhit)) (.ImpactPoint (Collision|BreakHitResult _outhit)) (.TraceEnd (Collision|BreakHitResult _outhit))) (CallFunction|GetMuzzleSocketLocation)))))

(fn GetMuzzleSocketLocation
  (return (Transformation|GetSocketLocation (Variables|Default|GetMuzzleScene) (Variables|Default|GetMuzzleSocketName))))

(fn CalculateTimeBetweenShots
  (bind _output_get (LocalVariables|SetL_TimeToShoot (/ 1.0 (.RateOfFire (Utilities|Struct|BreakSTRUCT_WeaponStats (Variables|Default|GetWeaponStats))))))
  (return _output_get))

(fn StopShooting
  (bind _timebetweenshots (CallFunction|CalculateTimeBetweenShots))
  (Utilities|Time|SetTimerbyEvent (EventDispatchers|CreateEvent :!event MakeShot) _timebetweenshots))