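; AI controller for BP_NPC_Base pawns that runs the BT_Main behavior tree on BeginPlay.
; AI perception updates write the sensed actor to a blackboard key and clear it when sensing fails.
; Tick prints that key's actor and the last stimulus's sense class and age as on-screen debug.
; CreateTargetPointsArray is an unfinished stub that only finds and counts BP_ZombieTargetPoint actors.
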(event OnTargetPerceptionUpdated(AIPerception)
  (params (Actor :type Actor%20Object%20Reference) (Stimulus :type AI%20Stimulus%20Structure))
  (Utilities|IsValid Actor
    (:Is%20Valid
      (Variables|Default|SetOtherActor Actor)
      (Variables|Default|SetStimulus Stimulus)
      (if (Utilities|Struct|BreakAIStimulus (Variables|Default|GetStimulus))
        (AI|Components|Blackboard|SetValueasObject (Variables|Default|GetBlackboard) (Variables|Default|GetBBOtherActorKey) (Variables|Default|GetOtherActor))
        (else
          (AI|Components|Blackboard|SetValueasObject (Variables|Default|GetBlackboard) (Variables|Default|GetBBOtherActorKey) 0))))))

(event EventBeginPlay
  (bind _returnvalue (Pawn|GetControlledPawn))
  (Utilities|IsValid _returnvalue
    (:Is%20Valid
      (bind _asbp_npc_base (Utilities|Casting|CastToBP_NPC_Base _returnvalue))
      (Variables|Default|SetControlledPawn _asbp_npc_base)
      (AI|RunBehaviorTree "/Game/Characters/NPCs/BT_Main.BT_Main"))))

(event EventTick
  (params (DeltaSeconds :type Float%20%28single-precision%29))
  (Development|PrintString (Utilities|GetDisplayName (AI|Components|Blackboard|GetValueasObject (Variables|Default|GetBlackboard) (Variables|Default|GetBBOtherActorKey))) true true "(R=0.000000,G=0.660000,B=1.000000,A=1.000000)" DeltaSeconds)
  (bind _returnvalue (Class|AIPerceptionSystem|GetSenseClassforStimulus (Variables|Default|GetStimulus)))
  (Development|PrintString (Utilities|String|Append (Utilities|GetClassDisplayName _returnvalue) "||||" (Utilities|String|ToString(Float) (.Age (Utilities|Struct|BreakAIStimulus (Variables|Default|GetStimulus))))) true true "(R=0.000000,G=0.660000,B=1.000000,A=1.000000)" DeltaSeconds))

(fn ConstructionScript)

(fn CreateTargetPointsArray
  (bind _outactors (Actor|GetAllActorsOfClass "/Game/Characters/NPCs/BP_ZombieTargetPoint.BP_ZombieTargetPoint_C"))
  (LocalVariables|SetL_MaxCount (Utilities|Array|Length _outactors)))