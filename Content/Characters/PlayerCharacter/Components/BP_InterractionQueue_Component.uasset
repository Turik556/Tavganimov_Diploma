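; Player character component that queues interactable actors with their properties and sends an interact message to one on demand.
; Interact picks the actor in sight, or the first queued one if none, and requires a sight match for entries flagged IsNeedSight.
; Tick runs a camera line trace with debug output, switched on by sight-required entries.
; A successful interaction either stops tick (sight entries) or dequeues the actor (others).
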(event Custom|CustomEvent_0
  (Components|Tick|SetComponentTickEnabled false))

(event EventBeginPlay
  (CallFunction|SetOwner)
  (Components|Tick|SetComponentTickEnabled false))

(event EventTick
  (params (DeltaSeconds :type Float%20%28single-precision%29))
  (CallFunction|SetActorinSight)
  (CallFunction|Debug DeltaSeconds)
  (EventDispatchers|BindEventtoOnNeedSightRemoved (delegate Custom|CustomEvent_0)))

(fn Debug
  (params (Duration :type Float%20%28single-precision%29))
  (bind _keys (Utilities|Map|Keys (Variables|Default|GetInteractQueue)))
  (for _array_element _keys
    (Development|PrintString (Utilities|GetDisplayName _array_element) true true "(R=0.000000,G=0.270833,B=0.036676,A=1.000000)" Duration)
    (Development|PrintString (Utilities|GetDisplayName (Variables|Default|GetActorInSight)) true true "(R=1.000000,G=0.000000,B=0.017848,A=1.000000)" Duration)))

(fn SetActorinSight
  (bind _returnvalue (Components|GetOwner))
  (bind _returnvalue_2 (Actor|GetComponentbyClass _returnvalue "/Script/Engine.CameraComponent"))
  (Utilities|IsValid _returnvalue_2
    (:Is%20Valid
      (LocalVariables|SetL_Camera _returnvalue_2)
      (bind _l_camera (LocalVariables|GetL_Camera)
        (:then
          (bind _desiredview (Class|CameraComponent|GetCameraView _l_camera 0.0))
          (LocalVariables|SetL_CameraLocation (Utilities|Struct|BreakMinimalViewInfo _desiredview))
          (bind _outhit (Collision|LineTraceByChannel (LocalVariables|GetL_CameraLocation) (+ (LocalVariables|GetL_CameraLocation) (* (Math|Vector|GetForwardVector (LocalVariables|GetL_Camera)) 5e+02)) "TraceTypeQuery1" false (Utilities|Array|MakeArray (Components|GetOwner)) "ForDuration" true "(R=1.000000,G=0.000000,B=0.000000,A=1.000000)" "(R=0.000000,G=1.000000,B=0.000000,A=1.000000)" 1.0))
          (Utilities|IsValid (.HitActor (Collision|BreakHitResult _outhit))
            (:Is%20Valid
              (bind _output_get (Variables|Default|SetActorInSight (.HitActor (Collision|BreakHitResult _outhit))))
              (Utilities|IsValid _output_get
                (:Is%20Not%20Valid
                  (Variables|Default|SetActorInSight 0))))
            (:Is%20Not%20Valid
              (Variables|Default|SetActorInSight 0))))
        (:else
          (return))))
    (:Is%20Not%20Valid
      (return))))

(fn SetOwner
  (bind _returnvalue (Components|GetOwner))
  (Utilities|IsValid _returnvalue
    (:Is%20Valid
      (Variables|Default|SetOwner _returnvalue))))

(fn GetStruct
  (params (OtherActor :type Actor%20Object%20Reference))
  (bind _interactqueue (Variables|Default|GetInteractQueue))
  (bind (_value _returnvalue) (Utilities|Map|Find _interactqueue OtherActor))
  (Utilities|IsValid OtherActor
    (:Is%20Valid
      (if _returnvalue
        (return _value true)
        (else
          (return "" false))))
    (:Is%20Not%20Valid
      (return "" false))))

(fn AddtoQueue
  (params (OtherActor :type Actor%20Object%20Reference) (Properties :type STRUCT%20Interact%20Item%20Properties%20Structure))
  (Utilities|IsValid OtherActor
    (:Is%20Valid
      (Utilities|IsinQueue OtherActor
        (:true
          (return false))
        (:false
          (Utilities|Map|Add (Variables|Default|GetInteractQueue) OtherActor Properties)
          (if (.IsNeedSight (Utilities|Struct|BreakSTRUCT_InteractItemProperties Properties))
            (Components|Tick|SetComponentTickEnabled true))
          (Default|CallOnAddedActor OtherActor)
          (return true))))
    (:Is%20Not%20Valid
      (return false))))

(fn Interact
  (Utilities|IsQueueValid
    (:true
      (bind _keys (Utilities|Map|Keys (Variables|Default|GetInteractQueue)))
      (LocalVariables|SetL_ArrayOfKeys _keys)
      (Variables|Default|SetIndex (Math|Integer|SelectInt (Utilities|Array|FindItem (LocalVariables|GetL_ArrayOfKeys) (Variables|Default|GetActorInSight)) 0 (Utilities|IsValid (Variables|Default|GetActorInSight))))
      (if (Utilities|Array|IsValidIndex (LocalVariables|GetL_ArrayOfKeys) (Variables|Default|GetIndex))
        (bind _output_get (LocalVariables|SetL_CurrentActor (Utilities|Array|Get(acopy) (LocalVariables|GetL_ArrayOfKeys) (Variables|Default|GetIndex))))
        (bind (_value _success) (CallFunction|GetStruct _output_get))
        (if _success
          (if (.IsNeedSight (Utilities|Struct|BreakSTRUCT_InteractItemProperties _value))
            (if (== (Variables|Default|GetActorInSight) (LocalVariables|GetL_CurrentActor))
              (bind _success_2 (Class|BPIInteract|Interact(Message) (LocalVariables|GetL_CurrentActor) (Variables|Default|GetOwner)))
              (if _success_2
                (Variables|Default|SetActorInSight 0)
                (Components|Tick|SetComponentTickEnabled false)
                (return true)
                (else
                  (return true)))
              (else
                (return false)))
            (else
              (bind _success_3 (Class|BPIInteract|Interact(Message) (LocalVariables|GetL_CurrentActor) (Variables|Default|GetOwner)))
              (if _success_3
                (bind _success_4 (CallFunction|RemovefromQueue (LocalVariables|GetL_CurrentActor)))
                (return _success_4)
                (else
                  (return true))))))))
    (:false
      (return false))))

(fn RemovefromQueue
  (params (OtherActor :type Actor%20Object%20Reference))
  (Utilities|IsValid OtherActor
    (:Is%20Valid
      (Utilities|IsinQueue OtherActor
        (:true
          (bind _returnvalue (Utilities|Map|Remove (Variables|Default|GetInteractQueue) OtherActor))
          (if (not (CallFunction|IsNeedSightinQueue))
            (Default|CallOnNeedSightRemoved))
          (Default|CallOnRemovedActor OtherActor)
          (return _returnvalue))
        (:false
          (return false))))
    (:Is%20Not%20Valid
      (return false))))

(fn IsNeedSightinQueue
  (bind _keys (Utilities|Map|Keys (Variables|Default|GetInteractQueue)))
  (bind _array_element (Utilities|Array|ForEachLoopwithBreak _keys :!label _label)
    (:LoopBody
      (bind _value (CallFunction|GetStruct _array_element))
      (if (.IsNeedSight (Utilities|Struct|BreakSTRUCT_InteractItemProperties _value))
        (Math|Integer|IncrementInt (LocalVariables|GetL_Increment)
          (:%20%20
            (goto _label Break)))))
    (:Completed
      (if (> (LocalVariables|GetL_Increment) 0)
        (return true)
        (else
          (return false))))))