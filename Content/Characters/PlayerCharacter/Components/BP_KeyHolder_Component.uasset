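; Player character component that tracks which key types are held, stored as a collection of enum values without duplicates.
; AddKey and RemoveKey use HasKey to validate changes, return whether they succeeded, and fire OnKeyAdded or OnKeyRemoved on success.
; Tick runs a Debug function every frame that prints each held key on screen, using DeltaSeconds as the message duration.
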(event EventBeginPlay)

(event EventTick
  (params (DeltaSeconds :type Float%20%28single-precision%29))
  (CallFunction|Debug DeltaSeconds))

(fn AddKey
  (params (KeyType :type ENUM_KeyType%20Enum%20%28by%20ref%29 :default "NewEnumerator0"))
  (if (CallFunction|HasKey KeyType)
    (return false)
    (else
      (Utilities|Array|AddUnique (Variables|Default|GetKeyHolder) KeyType)
      (Default|CallOnKeyAdded KeyType)
      (return true))))

(fn RemoveKey
  (params (KeyType :type ENUM_KeyType%20Enum%20%28by%20ref%29 :default "NewEnumerator0"))
  (if (CallFunction|HasKey KeyType)
    (bind _returnvalue (Utilities|Array|RemoveItem (Variables|Default|GetKeyHolder) KeyType))
    (if _returnvalue
      (Default|CallOnKeyRemoved KeyType)
      (return true)
      (else
        (return false)))
    (else
      (return false))))

(fn HasKey
  (params (KeyType :type ENUM_KeyType%20Enum%20%28by%20ref%29 :default "NewEnumerator0"))
  (return (Utilities|Array|ContainsItem (Variables|Default|GetKeyHolder) KeyType)))

(fn Debug
  (params (InputPin :type Float%20%28single-precision%29))
  (for _array_element (Variables|Default|GetKeyHolder)
    (Development|PrintString (Utilities|String|EnumtoString _array_element) true true "(R=1.000000,G=0.000000,B=0.056108,A=1.000000)" InputPin)))