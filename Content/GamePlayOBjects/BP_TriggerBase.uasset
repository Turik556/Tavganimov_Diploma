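; Base trigger volume that reacts when the player character enters its collision box.
; Begin overlap accepts only an exact BP_PlayerCharacter class match, stores it as OverlappedActor and calls OverlappEffect, a stub that just returns true.
; End overlap clears OverlappedActor whichever actor leaves.
; The construction script sizes the box from BoxExtent and lifts it by its Z extent so its bottom sits at its parent's origin.
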(event OnComponentBeginOverlap(CollisionBox)
  (params (OverlappedComponent :type Primitive%20Component%20Object%20Reference) (OtherActor :type Actor%20Object%20Reference) (OtherComp :type Primitive%20Component%20Object%20Reference) (OtherBodyIndex :type Integer) (bFromSweep :type Boolean) (SweepResult :type Hit%20Result%20Structure%20%28by%20ref%29))
  (Utilities|IsValid OtherActor
    (:Is%20Valid
      (if (== (Utilities|GetClass OtherActor) "/Game/Characters/PlayerCharacter/BP_PlayerCharacter.BP_PlayerCharacter_C")
        (Variables|Default|SetOverlappedActor OtherActor)
        (CallFunction|OverlappEffect)))))

(event OnComponentEndOverlap(CollisionBox)
  (params (OverlappedComponent :type Primitive%20Component%20Object%20Reference) (OtherActor :type Actor%20Object%20Reference) (OtherComp :type Primitive%20Component%20Object%20Reference) (OtherBodyIndex :type Integer))
  (Variables|Default|SetOverlappedActor 0))

(event EventBeginPlay)

(event Collision|EventActorBeginOverlap
  (params (OtherActor :type Actor%20Object%20Reference)))

(event EventTick
  (params (DeltaSeconds :type Float%20%28single-precision%29)))

(fn ConstructionScript
  (Components|Box|SetBoxExtent (Variables|Default|GetCollisionBox) (Variables|Default|GetBoxExtent) true)
  (Transformation|SetRelativeLocation (Variables|Default|GetCollisionBox) (Math|Vector|MakeVector 0.0 0.0 (.Z (Math|Vector|BreakVector (Variables|Default|GetBoxExtent)))) false false))

(fn OverlappEffect
  (return true))