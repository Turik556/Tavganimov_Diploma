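; Key lock component for sliding doors that tracks a locked state and unlocks only for actors carrying the required key.
; Lock sets the state and fires a locked notification, while UnLock queries the actor's BP_KeyHolder_Component for RequiredKey before clearing it and notifying.
; Both return whether the state changed.
; Component activation calls Lock; deactivation calls UnLock without an actor, so that call cannot unlock.
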(event Custom|OnComponentActivated_Event
  (params (Component :type Actor%20Component%20Object%20Reference) (bReset :type Boolean))
  (CallFunction|Lock))

(event Custom|OnComponentDeactivated_Event
  (params (Component :type Actor%20Component%20Object%20Reference))
  (CallFunction|UnLock))

(fn Lock
  (if (Variables|Default|GetIsLocked)
    (return false)
    (else
      (Variables|Default|SetIsLocked true)
      (Default|CallOnLocked)
      (return true))))

(fn UnLock
  (params (OtherActor :type Actor%20Object%20Reference))
  (if (Variables|Default|GetIsLocked)
    (Utilities|IsValid OtherActor
      (:Is%20Valid
        (bind _output_get (LocalVariables|SetL_KeyHolderComponent (Actor|GetComponentbyClass OtherActor "/Game/Characters/PlayerCharacter/Components/BP_KeyHolder_Component.BP_KeyHolder_Component_C")))
        (Utilities|IsValid _output_get
          (:Is%20Valid
            (if (Default|HasKey (LocalVariables|GetL_KeyHolderComponent) (Variables|Default|GetRequiredKey))
              (Variables|Default|SetIsLocked false)
              (Default|CallOnUnlocked)
              (return true)
              (else
                (return false))))
          (:Is%20Not%20Valid
            (return false))))
      (:Is%20Not%20Valid
        _)))
  (return false))