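; Sliding door base that moves its mesh between an initial and target location, with optional key locking.
; A state enum (Open, Closed, Locked, Transition) drives a timeline that lerps the mesh, and calls mid-slide reverse direction.
; Open and Close share the same toggle logic, ignored while locked.
; The construction script previews the initial state, while lock and unlock delegate to BPKeyLockComponent, with optional opening on unlock.
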(event Custom|Open
  (Utilities|IsLocked
    (:false
      (Utilities|SwitchCurrentStateExec
        (:Open
          (CallFunction|SetTargetState "NewEnumerator1")
          (bind _progression (Timeline|DoorAnimation ReverseFromEnd)
            (:Update
              (CallFunction|AnimateDoor _progression))
            (:Finished
              (Variables|Default|SetCurrentState (Variables|Default|GetTargetState)))))
        (:Closed
          (CallFunction|SetTargetState "NewEnumerator0")
          (Timeline|DoorAnimation PlayFromStart))
        (:Transition
          (Utilities|SwitchTargetStateExec
            (:Open
              (Variables|Default|SetTargetState "NewEnumerator1")
              (Timeline|DoorAnimation Reverse))
            (:Closed
              (Variables|Default|SetTargetState "NewEnumerator0")
              (Timeline|DoorAnimation Play))))))))

(event Custom|Close
  (Utilities|IsLocked
    (:false
      (Utilities|SwitchCurrentStateExec
        (:Open
          (CallFunction|SetTargetState "NewEnumerator1")
          (bind _progression (Timeline|DoorAnimation ReverseFromEnd)
            (:Update
              (CallFunction|AnimateDoor _progression))
            (:Finished
              (Variables|Default|SetCurrentState (Variables|Default|GetTargetState)))))
        (:Closed
          (CallFunction|SetTargetState "NewEnumerator0")
          (Timeline|DoorAnimation PlayFromStart))
        (:Transition
          (Utilities|SwitchTargetStateExec
            (:Open
              (Variables|Default|SetTargetState "NewEnumerator1")
              (Timeline|DoorAnimation Reverse))
            (:Closed
              (Variables|Default|SetTargetState "NewEnumerator0")
              (Timeline|DoorAnimation Play))))))))

(event EventBeginPlay)

(event Collision|EventActorBeginOverlap
  (params (OtherActor :type Actor%20Object%20Reference)))

(fn ConstructionScript
  (Variables|/Game/GamePlayOBjects/Doors/SlideDoor/BP_KeyLockComponent.BP_KeyLockComponent_C|SetRequiredKey (Variables|Default|GetBP_KeyLockComponent) (Variables|Default|GetRequiredKey))
  (bind _currentstate (CallFunction|SetInitialState))
  (CallFunction|SetInitialLocation)
  (CallFunction|AnimateDoor (Utilities|Select :Index _currentstate :NewEnumerator0 1.0 :NewEnumerator1 0.0 :NewEnumerator3 0.0 :NewEnumerator2 1.0))
  (Utilities|IsInitialState "NewEnumerator3"
    (:true
      (Variables|/Game/GamePlayOBjects/Doors/SlideDoor/BP_KeyLockComponent.BP_KeyLockComponent_C|SetIsLocked (Variables|Default|GetBP_KeyLockComponent) true))))

(fn IsCurrentState
  (params (State :type ENUM_DoorStates%20Enum :default "NewEnumerator0"))
  (return (Utilities|Enum|Equal(Enum) State (Variables|Default|GetCurrentState))))

(fn IsTargetState
  (params (State :type ENUM_DoorStates%20Enum :default "NewEnumerator0"))
  (return (Utilities|Enum|Equal(Enum) State (Variables|Default|GetTargetState))))

(fn SetTargetState
  (params (TargetState :type ENUM_DoorStates%20Enum :default "NewEnumerator0"))
  (Variables|Default|SetTargetState TargetState)
  (Variables|Default|SetCurrentState "NewEnumerator2"))

(fn SetCurrentState
  (params (CurrentState :type ENUM_DoorStates%20Enum :default "NewEnumerator0"))
  (Variables|Default|SetCurrentState CurrentState))

(fn AnimateDoor
  (params (Alpha :type Float%20%28single-precision%29))
  (Transformation|SetRelativeLocation (Variables|Default|GetDoorMesh) (Math|Vector|Lerp(Vector) (Variables|Default|GetInitialLocation) (Variables|Default|GetTargetLocation) Alpha) false false))

(fn SetInitialLocation
  (Variables|Default|SetInitialLocation (Variables|/Script/Engine.SceneComponent|GetRelativeLocation (Variables|Default|GetDoorMesh))))

(fn SetInitialState
  (Utilities|IsInitialState "NewEnumerator2"
    (:true
      (Variables|Default|SetInitialState "NewEnumerator1"))
    (:false
      _))
  (bind _output_get (Variables|Default|SetCurrentState (Variables|Default|GetInitialState)))
  (return _output_get))

(fn LockDoor
  (Utilities|IsLocked
    (:true
      (return false))
    (:false
      (bind _success (Default|Lock (Variables|Default|GetBP_KeyLockComponent)))
      (if _success
        (Variables|Default|SetCurrentState "NewEnumerator3")
        (return true)
        (else
          (return false))))))

(fn UnlockDoor
  (params (OtherActor :type Actor%20Object%20Reference) (OpenImideatly :type Boolean))
  (Utilities|IsLocked
    (:true
      (bind _success (Default|UnLock (Variables|Default|GetBP_KeyLockComponent) OtherActor))
      (if _success
        (Variables|Default|SetCurrentState "NewEnumerator1")
        (if OpenImideatly
          (CallFunction|Open))
        (return true)
        (else
          (return false))))
    (:false
      (return false))))