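; BP_SlideDoorInterract is a sliding door that actors open through the interaction system.
; Its collision box adds the door, with its Properties, to the BP_InterractionQueue_Component of any overlapping actor that has one, and removes it when the overlap ends.
; Interact calls Open, then returns whether CurrentState matches one particular enum state.
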(event OnComponentBeginOverlap(CollisionBox)
  (params (OverlappedComponent :type Primitive%20Component%20Object%20Reference) (OtherActor :type Actor%20Object%20Reference) (OtherComp :type Primitive%20Component%20Object%20Reference) (OtherBodyIndex :type Integer) (bFromSweep :type Boolean) (SweepResult :type Hit%20Result%20Structure%20%28by%20ref%29))
  (bind _returnvalue (Actor|GetComponentbyClass OtherActor "/Game/Characters/PlayerCharacter/Components/BP_InterractionQueue_Component.BP_InterractionQueue_Component_C"))
  (Utilities|IsValid OtherActor
    (:Is%20Valid
      (Utilities|IsValid _returnvalue
        (:Is%20Valid
          (Default|AddtoQueue _returnvalue self (Variables|Default|GetProperties)))))))

(event OnComponentEndOverlap(CollisionBox)
  (params (OverlappedComponent :type Primitive%20Component%20Object%20Reference) (OtherActor :type Actor%20Object%20Reference) (OtherComp :type Primitive%20Component%20Object%20Reference) (OtherBodyIndex :type Integer))
  (bind _returnvalue (Actor|GetComponentbyClass OtherActor "/Game/Characters/PlayerCharacter/Components/BP_InterractionQueue_Component.BP_InterractionQueue_Component_C"))
  (Utilities|IsValid OtherActor
    (:Is%20Valid
      (Utilities|IsValid _returnvalue
        (:Is%20Valid
          (Default|RemovefromQueue _returnvalue self))))))

(event EventBeginPlay
  (|CallParentFunction) ; This node is disabled and will not be called.\nDrag off pins to build functionality.
)

(event Collision|EventActorBeginOverlap
  (params (OtherActor :type Actor%20Object%20Reference))
  (|CallParentFunction OtherActor) ; This node is disabled and will not be called.\nDrag off pins to build functionality.
)

(event EventTick
  (params (DeltaSeconds :type Float%20%28single-precision%29)))

(fn ConstructionScript
  (|CallParentFunction))

(fn Interact
  (params (Actor :type Actor%20Object%20Reference))
  (CallFunction|Open)
  (if (Utilities|Enum|Equal(Enum) (Variables|Default|GetCurrentState) "NewEnumerator1")
    (return true)
    (else
      (return false))))