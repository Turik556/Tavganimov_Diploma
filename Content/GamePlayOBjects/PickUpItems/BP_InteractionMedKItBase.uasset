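; Base medkit pickup actor that restores health to the actor that interacts with it.
; Interact calls PickUpEffect, which finds the actor's BP_HeathComponent and increases it by the item's Value with clamping flagged off.
; The medkit destroys itself and reports success only when that increase succeeds, otherwise it stays in the world.
; Its event graph holds only disabled default events.
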(event EventBeginPlay
  (|CallParentFunction) ; This node is disabled and will not be called.\nDrag off pins to build functionality.
)

(event Collision|EventActorBeginOverlap
  (params (OtherActor :type Actor%20Object%20Reference))
  (|CallParentFunction OtherActor) ; This node is disabled and will not be called.\nDrag off pins to build functionality.
)

(event EventTick
  (params (DeltaSeconds :type Float%20%28single-precision%29))
  (|CallParentFunction DeltaSeconds) ; This node is disabled and will not be called.\nDrag off pins to build functionality.
)

(fn ConstructionScript
  (|CallParentFunction))

(fn PickUpEffect
  (params (Actor :type Actor%20Object%20Reference))
  (bind _returnvalue (Actor|GetComponentbyClass Actor "/Game/Components/BP_HeathComponent.BP_HeathComponent_C"))
  (Utilities|IsValid Actor
    (:Is%20Valid
      (Utilities|IsValid _returnvalue
        (:Is%20Valid
          (bind _success (Default|IncreaseValue _returnvalue false (Variables|Default|GetValue)))
          (return _success))))))

(fn Interact
  (params (Actor :type Actor%20Object%20Reference))
  (bind _success (CallFunction|PickUpEffect Actor))
  (if _success
    (Actor|DestroyActor)
    (return true)
    (else
      (return false))))