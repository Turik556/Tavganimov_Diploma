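; Base actor for interactable pickup items that are destroyed when successfully picked up.
; Its sphere overlap adds or removes it from the other actor's BP_InterractionQueue_Component, toggling the interact widget on success.
; Interact calls PickUpEffect, which returns true here as an apparent hook for children, and destroys the item on success.
; SetWidgetVisibility flips current state and also runs at construction; the DT_InteractItems lookup for ItemProperties is disconnected.
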(event OnComponentBeginOverlap(SphereCollision)
  (params (OverlappedComponent :type Primitive%20Component%20Object%20Reference) (OtherActor :type Actor%20Object%20Reference) (OtherComp :type Primitive%20Component%20Object%20Reference) (OtherBodyIndex :type Integer) (bFromSweep :type Boolean) (SweepResult :type Hit%20Result%20Structure%20%28by%20ref%29))
  (bind _returnvalue (Actor|GetComponentbyClass OtherActor "/Game/Characters/PlayerCharacter/Components/BP_InterractionQueue_Component.BP_InterractionQueue_Component_C"))
  (Utilities|IsValid OtherActor
    (:Is%20Valid
      (Utilities|IsValid _returnvalue
        (:Is%20Valid
          (bind _success (Default|AddtoQueue _returnvalue self (Variables|Default|GetItemProperties)))
          (if _success
            (CallFunction|SetWidgetVisibility)))))))

(event OnComponentEndOverlap(SphereCollision)
  (params (OverlappedComponent :type Primitive%20Component%20Object%20Reference) (OtherActor :type Actor%20Object%20Reference) (OtherComp :type Primitive%20Component%20Object%20Reference) (OtherBodyIndex :type Integer))
  (bind _returnvalue (Actor|GetComponentbyClass OtherActor "/Game/Characters/PlayerCharacter/Components/BP_InterractionQueue_Component.BP_InterractionQueue_Component_C"))
  (Utilities|IsValid OtherActor
    (:Is%20Valid
      (Utilities|IsValid _returnvalue
        (:Is%20Valid
          (bind _success (Default|RemovefromQueue _returnvalue self))
          (if _success
            (CallFunction|SetWidgetVisibility)))))))

(event EventBeginPlay
  (|CallParentFunction) ; This node is disabled and will not be called.\nDrag off pins to build functionality.
)

(event Collision|EventActorBeginOverlap
  (params (OtherActor :type Actor%20Object%20Reference)))

(event EventTick
  (params (DeltaSeconds :type Float%20%28single-precision%29))
  (|CallParentFunction DeltaSeconds) ; This node is disabled and will not be called.\nDrag off pins to build functionality.
)

(fn ConstructionScript
  (|CallParentFunction)
  (CallFunction|SetWidgetVisibility))

(fn PickUpEffect
  (params (Actor :type Actor%20Object%20Reference))
  (return true))

(fn SetWidgetVisibility
  (bind _interactwidget (Variables|Default|GetInteractWidget)
    (:then
      (if (not (Rendering|IsVisible _interactwidget))
        (Rendering|SetVisibility (Variables|Default|GetInteractWidget) true true)
        (else
          (Rendering|SetVisibility (Variables|Default|GetInteractWidget) false true))))
    (:else)))

(fn Interact
  (params (Actor :type Actor%20Object%20Reference))
  (bind _success (CallFunction|PickUpEffect Actor))
  (if _success
    (Actor|DestroyActor)
    (return true)
    (else
      (return false))))