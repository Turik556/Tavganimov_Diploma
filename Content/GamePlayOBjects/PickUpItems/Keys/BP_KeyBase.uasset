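; BP_KeyBase is the base key pickup, which gives its key type to the actor that interacts with it.
; Its construction script sets the mesh material by looking up the key type in a material map.
; Interact runs through Interaction to PickUpEffect, which finds the actor's BP_KeyHolder_Component and calls AddKey.
; A successful add triggers InteractionEnds, and the event graph holds only disabled default events.
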(event EventBeginPlay
  (|CallParentFunction) ; This node is disabled and will not be called.\nDrag off pins to build functionality.
)

(event Collision|EventActorBeginOverlap
  (params (OtherActor :type Actor%20Object%20Reference)))

(event EventTick
  (params (DeltaSeconds :type Float%20%28single-precision%29))
  (|CallParentFunction DeltaSeconds) ; This node is disabled and will not be called.\nDrag off pins to build functionality.
)

(fn ConstructionScript
  (|CallParentFunction)
  (Rendering|Material|SetMaterial (Variables|Default|GetItemMesh) 0 (Utilities|ResolveSoftReference (.Value (Utilities|Map|Find (Variables|Default|GetKeyMaterials) (Variables|Default|GetKeyType))))))

(fn Interact
  (params (Actor :type Actor%20Object%20Reference))
  (bind _success (CallFunction|Interaction Actor))
  (if _success
    (CallFunction|InteractionEnds)
    (return false)))

(fn Interaction
  (params (Actor :type Actor%20Object%20Reference))
  (Utilities|IsValid Actor
    (:Is%20Valid
      (bind _success (CallFunction|PickUpEffect Actor))
      (if _success
        (return true)
        (else
          (return false))))))

(fn PickUpEffect
  (params (TargetActor :type Actor%20Object%20Reference))
  (Utilities|IsValid TargetActor
    (:Is%20Valid
      (bind _output_get (LocalVariables|SetL_KeyHolder (Actor|GetComponentbyClass TargetActor "/Game/Characters/PlayerCharacter/Components/BP_KeyHolder_Component.BP_KeyHolder_Component_C")))
      (Utilities|IsValid _output_get
        (:Is%20Valid
          (bind _success (Default|AddKey (LocalVariables|GetL_KeyHolder) (Variables|Default|GetKeyType)))
          (if _success
            (return true)))
        (:Is%20Not%20Valid
          (return false))))
    (:Is%20Not%20Valid
      (return false))))