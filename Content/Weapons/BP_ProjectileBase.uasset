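; Base projectile actor that launches along MovementDirection at its initial speed and damages NPCs on impact.
; On hit it prints the other actor's name, applies DamageValue through BP_DamageObject only if the class is exactly BP_NPC_Base, then destroys itself.
; SetTargetLocation runs a debug-drawn camera trace with its result unused.
; SpawnDecal only spawns an emitter; neither helper is called here.
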(event EventBeginPlay
  (Variables|/Script/Engine.MovementComponent|SetVelocity (Variables|Default|GetProjectileMovement) (* (Variables|Default|GetMovement%20Direction) (Variables|/Script/Engine.ProjectileMovementComponent|GetInitialSpeed (Variables|Default|GetProjectileMovement)))))

(event Collision|EventHit
  (params (MyComp :type Primitive%20Component%20Object%20Reference) (Other :type Actor%20Object%20Reference) (OtherComp :type Primitive%20Component%20Object%20Reference) (bSelfMoved :type Boolean) (HitLocation :type Vector :default "0, 0, 0") (HitNormal :type Vector :default "0, 0, 0") (NormalImpulse :type Vector :default "0, 0, 0") (Hit :type Hit%20Result%20Structure%20%28by%20ref%29))
  (Development|PrintString (Utilities|GetDisplayName Other))
  (if (== (Utilities|GetClass Other) "/Game/Characters/BP_NPC_Base.BP_NPC_Base_C")
    (Game|Damage|ApplyDamage Other (Math|Conversions|ToFloat(Integer) (Variables|Default|GetDamageValue)) 0 0 "/Game/Blueprints/Objects/BP_DamageObject.BP_DamageObject_C"))
  (Actor|DestroyActor))

(event EventTick
  (params (DeltaSeconds :type Float%20%28single-precision%29)))

(fn ConstructionScript)

(fn SetTargetLocation
  (bind _returnvalue (Game|GetPlayerCharacter 0))
  (Utilities|IsValid _returnvalue
    (:Is%20Valid
      (bind _asbp_player_character (Utilities|Casting|CastToBP_PlayerCharacter _returnvalue))
      (bind _desiredview (Class|CameraComponent|GetCameraView (Variables|/Game/Characters/PlayerCharacter/BP_PlayerCharacter.BP_PlayerCharacter_C|GetCamera _asbp_player_character) 0.0))
      (bind _outhit (Collision|LineTraceByChannel (Utilities|Struct|BreakMinimalViewInfo _desiredview) (+ (Utilities|Struct|BreakMinimalViewInfo _desiredview) (* (Math|Vector|GetForwardVector (Variables|/Game/Characters/PlayerCharacter/BP_PlayerCharacter.BP_PlayerCharacter_C|GetCamera _asbp_player_character)) 5e+03)) "TraceTypeQuery2" false 0 "ForDuration")))))

(fn SpawnDecal
  (params (Hit :type Hit%20Result%20Structure))
  (Effects|SpawnEmitteratLocation 0 "0, 0, 0"))